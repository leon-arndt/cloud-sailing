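; BP_Harpoon_VR is a VR harpoon launcher that can be grabbed, aimed and fired.
; Pickup uses the caller's physics handle to grab the rigged mesh's vertical-rotation bone at the attach component's location, and Drop releases it.
; A projectile is spawned and snapped to ProjectileLocation on BeginPlay.
; Left mouse fires it through a DoOnce, then after a short delay resets the gate and loads a new projectile.
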(event `/Game/VirtualRealityBP/Blueprints/PickupActorInterface.Pickup`
  (params (AttachTo :type "SceneComponent Object Reference") (PH :type "PhysicsHandleComponent Object Reference") (BoneName :type Name))
  (bind _returnvalue_location (`KismetMathLibrary.BreakTransform` (`SceneComponent.K2_GetComponentToWorld` AttachTo)))
  (set `self.PH` PH)
  (`PhysicsHandleComponent.GrabComponentAtLocation` PH (`self.harpoon_blocking_rigged`) "jt_rotate_vertical" _returnvalue_location))

(event `/Game/VirtualRealityBP/Blueprints/PickupActorInterface.Drop`
  (`KismetSystemLibrary.PrintString` "drop")
  (`PhysicsHandleComponent.ReleaseComponent` (`self.PH`)))

(event `Key|LeftMouseButton`
  (params (Key :type "Key Structure"))
  (:`Pressed`
    (`/Engine/EditorBlueprintResources/StandardMacros.DoOnce` false :!label _label
      (:`Completed`
        (`/Game/Blueprints/BP_Harpoon_projectile.Fire` (`self.Loaded_Projectile`) (0.0 0.0 0.0))
        (`KismetSystemLibrary.Delay` 1.0)
        (`self.ResetProjectile`)))))

(event `ResetProjectile`
  (`|ExecutionSequence`
    (:`then_0`
      (goto _label :!via `Reset`))
    (:`then_1`
      (bind _returnvalue (`|SpawnActorFromClass` "/Game/Blueprints/BP_Harpoon_projectile.BP_Harpoon_projectile_C" (`SceneComponent.K2_GetComponentToWorld` (`self.Projectile_location`)) "Undefined" "OverrideRootScale" null null :!label _label_2))
      (bind _output_get (set `self.Loaded_Projectile` _returnvalue))
      (`self.K2_AttachToComponent` _output_get (`self.Projectile_location`) "None" "SnapToTarget" "SnapToTarget" "SnapToTarget" true))))

(event `self.ReceiveBeginPlay`
  (goto _label_2))

(fn `UserConstructionScript`)