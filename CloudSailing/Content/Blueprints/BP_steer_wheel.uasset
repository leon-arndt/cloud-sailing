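; VR steering wheel that lets motion controllers steer a BP_ShipController2 ship and change its speed.
; Pickup grabs the rigged mesh's wheel bone with a tuned physics handle, and Drop releases it.
; Tick turns bone yaw into smoothed steering input, mirrors it on a visible wheel mesh, and snaps the actor to the ship's WheelLocation.
; Motion controllers overlapping two cubes raise or lower ship speed in fixed steps.
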(event `self.Cube.OnComponentBeginOverlap`
  (params (OverlappedComponent :type "PrimitiveComponent Object Reference") (OtherActor :type "Actor Object Reference") (OtherComp :type "PrimitiveComponent Object Reference") (OtherBodyIndex :type Integer) (bFromSweep :type Boolean) (SweepResult :type "HitResult Structure (by ref)"))
  (bind _ship (`self.ship`))
  (cast `/Game/VirtualRealityBP/Blueprints/BP_MotionController` OtherActor)
  (set `/Game/Blueprints/BP_ShipController2.Speed` (+ (`/Game/Blueprints/BP_ShipController2.Speed` _ship) 5.0) _ship))

(event `self.Cube1.OnComponentBeginOverlap`
  (params (OverlappedComponent :type "PrimitiveComponent Object Reference") (OtherActor :type "Actor Object Reference") (OtherComp :type "PrimitiveComponent Object Reference") (OtherBodyIndex :type Integer) (bFromSweep :type Boolean) (SweepResult :type "HitResult Structure (by ref)"))
  (bind _ship (`self.ship`))
  (cast `/Game/VirtualRealityBP/Blueprints/BP_MotionController` OtherActor)
  (set `/Game/Blueprints/BP_ShipController2.Speed` (+ (`/Game/Blueprints/BP_ShipController2.Speed` _ship) -5.0) _ship))

(event `/Game/VirtualRealityBP/Blueprints/PickupActorInterface.Pickup`
  (params (AttachTo :type "SceneComponent Object Reference") (PH :type "PhysicsHandleComponent Object Reference") (BoneName :type Name) (Hand :type "EControllerHand Enum" :default "Left"))
  (bind _returnvalue_location (`KismetMathLibrary.BreakTransform` (`SceneComponent.K2_GetComponentToWorld` AttachTo)))
  (`PhysicsHandleComponent.SetLinearDamping` PH 20.0)
  (`PhysicsHandleComponent.SetLinearStiffness` PH 400.0)
  (`PhysicsHandleComponent.SetAngularDamping` PH 50.0)
  (`PhysicsHandleComponent.SetAngularStiffness` PH 0.0)
  (set `PhysicsHandleComponent.bInterpolateTarget` true PH)
  (if (`self.graped`)
    (`PhysicsHandleComponent.ReleaseComponent` (`self.PH`)))
  (set `self.graped` true)
  (set `self.PH` PH)
  (`PhysicsHandleComponent.GrabComponentAtLocation` PH (`self.harpoon_blocking_rigged`) "jt_steering_wheel" _returnvalue_location))

(event `/Game/VirtualRealityBP/Blueprints/PickupActorInterface.Drop`
  (params (Hand :type "EControllerHand Enum" :default "Left"))
  (set `self.graped` false)
  (`PhysicsHandleComponent.ReleaseComponent` (`self.PH`)))

(event `self.ReceiveBeginPlay`
  (bind _outactors (`GameplayStatics.GetAllActorsOfClass` "/Game/Blueprints/BP_ShipController2.BP_ShipController2_C"))
  (set `self.Ship` (`|GetArrayItem` _outactors)))

(event `self.ReceiveTick`
  (params (DeltaSeconds :type "Float (single-precision)"))
  (set `self.steer` (`KismetMathLibrary.FInterpTo` (`self.steer`) (/ (.yaw (.rotation (`KismetMathLibrary.ConvertTransformToRelative` (`SceneComponent.GetSocketTransform` (`self.harpoon_blocking_rigged`) "jt_steering_wheel" "RTS_World") (`self.GetTransform`)))) 190.0) (`GameplayStatics.GetWorldDeltaSeconds`) 1.0))
  (`/Game/Blueprints/BP_ShipController2.steer` (`self.Ship`) (`self.steer`))
  (set `self.lastSteerValue` (struct))
  (`SceneComponent.K2_SetRelativeRotation` (`self.SteeringWheel_Single`) (`KismetMathLibrary.MakeRotator` 0.0 (.yaw (.rotation (`KismetMathLibrary.ConvertTransformToRelative` (`SceneComponent.GetSocketTransform` (`self.harpoon_blocking_rigged`) "jt_steering_wheel" "RTS_World") (`self.GetTransform`))))) false false)
  (`self.K2_SetActorLocationAndRotation` (`SceneComponent.K2_GetComponentLocation` (`/Game/Blueprints/BP_ShipController2.wheelLocation` (`self.Ship`))) (`SceneComponent.K2_GetComponentRotation` (`/Game/Blueprints/BP_ShipController2.wheelLocation` (`self.Ship`)))))

(fn `UserConstructionScript`)