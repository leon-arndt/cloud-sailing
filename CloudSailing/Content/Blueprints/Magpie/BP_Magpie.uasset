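; AI-driven Magpie that leads the player's ship along indexed waypoints, taunting it when it falls behind.
; A recurring distance check switches between Taunt and GoToNextGoal, feeding state, goal and speed to a behavior tree through the blackboard.
; It speeds up as the ship nears, with a timed max-speed burst when overtaken toward the waypoint.
; Tick also turns the mesh toward movement and enlarges it with distance from the ship.
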(event `self.ReceiveTick`
  (params (DeltaSeconds :type "Float (single-precision)"))
  (bind (_returnvalue_x _returnvalue_y) (`KismetMathLibrary.BreakVector` (`self.K2_GetActorLocation`)))
  (bind (_returnvalue_x_2 _returnvalue_y_2) (`KismetMathLibrary.BreakVector` (`self.K2_GetActorLocation`)))
  (bind (_returnvalue_x_3 _returnvalue_y_3) (`KismetMathLibrary.BreakVector` (`self.K2_GetActorLocation` (`self.Ship`))))
  (bind (_returnvalue_x_4 _returnvalue_y_4) (`KismetMathLibrary.BreakVector` (`self.K2_GetActorLocation` (`self.CurrentWaypoint`))))
  (bind (_returnvalue_x_5 _returnvalue_y_5) (`KismetMathLibrary.BreakVector` (`self.K2_GetActorLocation` (`self.CurrentWaypoint`))))
  (bind (_returnvalue_x_6 _returnvalue_y_6) (`KismetMathLibrary.BreakVector` (`self.K2_GetActorLocation` (`self.Ship`))))
  (bind (_returnvalue_roll _returnvalue_pitch _returnvalue_yaw) (`KismetMathLibrary.BreakRotator` (`KismetMathLibrary.Conv_VectorToRotator` (- (`self.K2_GetActorLocation`) (`self.lastLocation`)))))
  (bind _returnvalue (`KismetMathLibrary.MapRangeClamped` (`KismetMathLibrary.VSize` (- (`self.K2_GetActorLocation` (`self.Ship`)) (`self.K2_GetActorLocation`))) 10000.0 100000.0 1.0 10.0))
  ;[1 1 1] rotate to movement
  (`SceneComponent.K2_SetWorldRotation` (`self.Magpie`) (`KismetMathLibrary.RInterpTo` (`SceneComponent.K2_GetComponentRotation` (`self.Magpie`)) (`KismetMathLibrary.MakeRotator` _returnvalue_roll _returnvalue_pitch (- _returnvalue_yaw 90.0)) (`GameplayStatics.GetWorldDeltaSeconds`) 1.0) false false)
  (set `self.lastLocation` (`self.K2_GetActorLocation`))
  (`|ExecutionSequence`
    (:`then_0`
      (`SceneComponent.SetWorldScale3D` (`self.Magpie`) (`KismetMathLibrary.MakeVector` _returnvalue _returnvalue _returnvalue)))
    (:`then_1`
      (`KismetSystemLibrary.Delay` 0.2)
      (set `self.Speed` (`KismetMathLibrary.MapRangeClamped` (`KismetMathLibrary.VSize` (- (`KismetMathLibrary.MakeVector` _returnvalue_x_3 _returnvalue_y_3) (`KismetMathLibrary.MakeVector` _returnvalue_x_2 _returnvalue_y_2))) 3000.0 100.0 50.0 (`self.maxSpeed`)))
      (switch `/Game/Blueprints/Magpie/MagpieState` (`self.MagpieState`)
        (:`NewEnumerator0`
          (`BlackboardComponent.SetValueAsFloat` (`AIBlueprintHelperLibrary.GetBlackboard` self) "Speed" (`self.maxSpeed`)))
        (:`NewEnumerator1`
          (if (< (`KismetMathLibrary.VSize` (- (`KismetMathLibrary.MakeVector` _returnvalue_x_5 _returnvalue_y_5) (`KismetMathLibrary.MakeVector` _returnvalue_x_6 _returnvalue_y_6))) (`KismetMathLibrary.VSize` (- (`KismetMathLibrary.MakeVector` _returnvalue_x_4 _returnvalue_y_4) (`KismetMathLibrary.MakeVector` _returnvalue_x _returnvalue_y))))
            _
            (elif (`self.FlyAhead`)
              _
              (else
                (`BlackboardComponent.SetValueAsFloat` (`AIBlueprintHelperLibrary.GetBlackboard` self) "Speed" (`self.Speed`))
                (goto _label :!via `Reset`))))
          (`BlackboardComponent.SetValueAsFloat` (`AIBlueprintHelperLibrary.GetBlackboard` self) "Speed" (`self.maxSpeed`))
          (`/Engine/EditorBlueprintResources/StandardMacros.DoOnce` false :!label _label
            (:`Completed`
              (set `self.FlyAhead` true)
              (`KismetSystemLibrary.Delay` 6.0)
              (set `self.FlyAhead` false))))))))

(event `manageState`
  (bind (_returnvalue_x _returnvalue_y _returnvalue_z) (`KismetMathLibrary.BreakVector` (`self.K2_GetActorLocation`)))
  (bind (_returnvalue_x_2 _returnvalue_y_2 _returnvalue_z_2) (`KismetMathLibrary.BreakVector` (`self.K2_GetActorLocation` (`self.Ship`))))
  (if (< (`KismetMathLibrary.VSize` (- (`KismetMathLibrary.MakeVector` _returnvalue_x_2 _returnvalue_y_2 _returnvalue_z_2) (`KismetMathLibrary.MakeVector` _returnvalue_x _returnvalue_y _returnvalue_z))) 1500.0)
    (`KismetSystemLibrary.Delay` 5.0)
    (`self.ChangeState` "NewEnumerator1")
    (`KismetSystemLibrary.Delay` (`self.TauntDelay`))
    (`self.manageState`)
    (else
      (`self.ChangeState` "NewEnumerator0")
      (`KismetSystemLibrary.Delay` 0.2)
      (`self.manageState`))))

(event `self.ReceiveBeginPlay`
  (`|ExecutionSequence`
    (:`then_0`
      (bind _outactors (`GameplayStatics.GetAllActorsOfClass` "/Game/Blueprints/BP_ShipController2.BP_ShipController2_C"))
      (set `self.Ship` (`|GetArrayItem` _outactors))
      (`AIController.RunBehaviorTree` (`AIBlueprintHelperLibrary.GetAIController` self) "/Game/Blueprints/Magpie/Magpie_BehaviorTree.Magpie_BehaviorTree")
      (`BlackboardComponent.SetValueAsObject` (`AIBlueprintHelperLibrary.GetBlackboard` self) "MagpieTauntLocationActor" (`self.TauntLocationObject`))
      (bind _outactors_2 (`GameplayStatics.GetAllActorsOfClass` "/Game/Blueprints/Magpie/MagpieWaypoint.MagpieWaypoint_C"))
      (bind _output_get (set `self.MagpieWayPoints` _outactors_2))
      (for _array_element _output_get
        (if (== (`/Game/Blueprints/Magpie/MagpieWaypoint.WaypointIndex` _array_element) (`self.GoalWayPointIndex`))
          (set `self.CurrentWaypoint` _array_element)
          (`BlackboardComponent.SetValueAsObject` (`AIBlueprintHelperLibrary.GetBlackboard` self) "MagpieGoalLocationActor" _array_element)
          (`BlackboardComponent.SetValueAsEnum` (`AIBlueprintHelperLibrary.GetBlackboard` self) "MagpieState" (`self.MagpieState`)))))
    (:`then_1`
      (`KismetSystemLibrary.Delay` 0.2)
      (`self.manageState`))))

(event `NextGoal`
  (`/Engine/EditorBlueprintResources/StandardMacros.IncrementInt` (`self.GoalWayPointIndex`)
    (:`  `
      (for _array_element (`self.MagpieWayPoints`)
        (if (== (`/Game/Blueprints/Magpie/MagpieWaypoint.WaypointIndex` _array_element) (`self.GoalWayPointIndex`))
          (`BlackboardComponent.SetValueAsObject` (`AIBlueprintHelperLibrary.GetBlackboard` self) "MagpieGoalLocationActor" _array_element)
          (set `self.CurrentWaypoint` _array_element))))))

(event `ChangeState`
  (params (newState :type "/Game/Blueprints/Magpie/MagpieState Enum" :default "NewEnumerator0"))
  (set `self.MagpieState` newState)
  (`BlackboardComponent.SetValueAsEnum` (`AIBlueprintHelperLibrary.GetBlackboard` self) "MagpieState" (`self.MagpieState`)))

(fn `UserConstructionScript`)