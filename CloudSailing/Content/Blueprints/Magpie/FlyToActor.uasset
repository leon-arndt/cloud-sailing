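; Behavior tree task for the Magpie that flies the SelfActor blackboard actor straight toward GoalActor.
; Each tick steps its location at constant speed using VInterpToConstant and the Speed key, with a clamped offset and a swept SetActorLocation.
; Execution finishes successfully after a zero-second delay, so each run moves only briefly and continued flight depends on the task being re-run.
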(event `self.ReceiveExecute`
  (params (OwnerActor :type "Actor Object Reference"))
  (`KismetSystemLibrary.Delay` 0.0)
  (`self.FinishExecute` true))

(event `self.ReceiveTick`
  (params (OwnerActor :type "Actor Object Reference") (DeltaSeconds :type "Float (single-precision)"))
  (bind _smothspeed (`self.SmothSpeed`))
  (bind _returnvalue (`Actor.K2_GetActorLocation` (`BTFunctionLibrary.GetBlackboardValueAsActor` (`self.SelfActor`))))
  (set `self.SmothSpeed` (`BTFunctionLibrary.GetBlackboardValueAsFloat` (`self.Speed`)))
  (`Actor.K2_SetActorLocation` (`BTFunctionLibrary.GetBlackboardValueAsActor` (`self.SelfActor`)) (+ _returnvalue (`KismetMathLibrary.ClampVectorSize` (- (`KismetMathLibrary.VInterpTo_Constant` _returnvalue (`Actor.K2_GetActorLocation` (`BTFunctionLibrary.GetBlackboardValueAsActor` (`self.GoalActor`))) (`GameplayStatics.GetWorldDeltaSeconds`) (`self.SmothSpeed`)) _returnvalue) (* _smothspeed -1.0) _smothspeed)) true false))