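; ShipFollower is an actor in the Magpie Blueprints that attaches itself to the player ship controller's sphere so that it moves with the ship.
; On BeginPlay it takes the first BP_ShipController2 found and attaches to its Sphere, keeping world transforms.
; The Cube overlap event is empty; disconnected leftover logic would move a taunting BP_Magpie to its next goal after a delay.
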(event `self.ReceiveBeginPlay`
  (bind _outactors (`GameplayStatics.GetAllActorsOfClass` "/Game/Blueprints/BP_ShipController2.BP_ShipController2_C"))
  (set `self.Ship` (`|GetArrayItem` _outactors))
  (`self.K2_AttachToComponent` (`/Game/Blueprints/BP_ShipController2.Sphere` (`self.Ship`)) "None" "KeepWorld" "KeepWorld" "KeepWorld" false))

(event `self.Cube.OnComponentBeginOverlap`
  (params (OverlappedComponent :type "PrimitiveComponent Object Reference") (OtherActor :type "Actor Object Reference") (OtherComp :type "PrimitiveComponent Object Reference") (OtherBodyIndex :type Integer) (bFromSweep :type Boolean) (SweepResult :type "HitResult Structure (by ref)")))

(fn `UserConstructionScript`)