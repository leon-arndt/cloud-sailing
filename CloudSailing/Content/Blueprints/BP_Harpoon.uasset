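; BP_Harpoon is a mouse-aimed harpoon launcher that fires on left click.
; Mouse X turns the Horizontal component's yaw, and inverted Mouse Y drives the Vertical component's roll.
; A BP_Harpoon_projectile spawns attached to ProjectileLocation at BeginPlay, ready to fire.
; A DoOnce gates each shot until, after a short delay, ResetProjectile re-arms it and loads a new projectile.
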(event `Key|LeftMouseButton`
  (params (Key :type "Key Structure"))
  (:`Pressed`
    (`/Engine/EditorBlueprintResources/StandardMacros.DoOnce` false :!label _label
      (:`Completed`
        (`/Game/Blueprints/BP_Harpoon_projectile.Fire` (`self.Loaded_Projectile`) (0.0 0.0 0.0))
        (`KismetSystemLibrary.Delay` 1.0)
        (`self.ResetProjectile`)))))

(event `ResetProjectile`
  (`|ExecutionSequence`
    (:`then_0`
      (goto _label :!via `Reset`))
    (:`then_1`
      (bind _returnvalue (`|SpawnActorFromClass` "/Game/Blueprints/BP_Harpoon_projectile.BP_Harpoon_projectile_C" (`SceneComponent.K2_GetComponentToWorld` (`self.Projectile_location`)) "Undefined" "OverrideRootScale" null null :!label _label_2))
      (bind _output_get (set `self.Loaded_Projectile` _returnvalue))
      (`self.K2_AttachToComponent` _output_get (`self.Projectile_location`) "None" "SnapToTarget" "SnapToTarget" "SnapToTarget" true))))

(event `self.ReceiveBeginPlay`
  (goto _label_2))

(event `InputAxisKey|MouseX`
  (params (AxisValue :type "Float (single-precision)"))
  (bind _horizontal (`self.Horizontal`))
  (bind (_returnvalue_roll _returnvalue_pitch _returnvalue_yaw) (`KismetMathLibrary.BreakRotator` (`SceneComponent.K2_GetComponentRotation` _horizontal)))
  (`SceneComponent.K2_SetWorldRotation` _horizontal (`KismetMathLibrary.MakeRotator` _returnvalue_roll _returnvalue_pitch (+ AxisValue _returnvalue_yaw)) false false))

(event `InputAxisKey|MouseY`
  (params (AxisValue :type "Float (single-precision)"))
  (bind _vertical (`self.Vertical`))
  (bind (_returnvalue_roll _returnvalue_pitch _returnvalue_yaw) (`KismetMathLibrary.BreakRotator` (`SceneComponent.K2_GetComponentRotation` _vertical)))
  (`SceneComponent.K2_SetWorldRotation` _vertical (`KismetMathLibrary.MakeRotator` (+ (* AxisValue -1.0) _returnvalue_roll) _returnvalue_pitch _returnvalue_yaw) false false))

(fn `UserConstructionScript`)