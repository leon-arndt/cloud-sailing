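; VR ship controller that plays theme music and wind, then moves the ship each tick until stopped.
; Tick drives forward and height-capped vertical movement, scaling a scene component with speed.
; The steer event turns and banks the ship, easing the turn out when stopped.
; Rotate adds cosine wave sway unless anti-motion-sickness mode is on, optionally counter-rotating the MotionControllerPawn to shield the player.
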(event `self.ReceiveBeginPlay`
  (`AkComponent.PostAkEvent` :`self` (`self.Ak`) :`AkEvent` "/Game/Audio/AkEvents/Play_mus_main_theme.Play_mus_main_theme")
  (`AkComponent.PostAkEvent` :`self` (`self.Ak`) :`AkEvent` "/Game/Audio/AkEvents/Play_amb_wind.Play_amb_wind")
  (bind _outactors (`GameplayStatics.GetAllActorsOfClass` "/Game/VirtualRealityBP/Blueprints/MotionControllerPawn.MotionControllerPawn_C"))
  (set `self.Player` (`|GetArrayItem` _outactors)))

(event `self.ReceiveTick`
  (params (DeltaSeconds :type "Float (single-precision)"))
  (bind _returnvalue (`KismetMathLibrary.MapRangeClamped` (`self.Speed`) 0.0 50.0 0.5 1.0))
  (if (not (`self.Stopded`))
    (`self.MoveForward` (`self.Speed`))
    (`self.MoveVertical` (`self.VerticalSpeed`))
    (`SceneComponent.SetRelativeScale3D` (`self.Scene`) (`KismetMathLibrary.MakeVector` _returnvalue 1.0 _returnvalue))))

(event `steer`
  (params (Value :type "Float (double-precision)"))
  (if (`self.Stopded`)
    (bind _output_get (set `self.lastSteer` (`KismetMathLibrary.FInterpTo` (`self.lastSteer`) 0.0 (`GameplayStatics.GetWorldDeltaSeconds`) 0.2)))
    (`self.Rotate` _output_get)
    (else
      (`self.Rotate` Value)
      (set `self.lastSteer` Value))))

(fn `MoveForward`
  (params (ForwardSpeed :type "Float (double-precision)"))
  (bind _returnvalue (* ForwardSpeed 0.7))
  (if (`self.Stopded`)
    (bind _output_get (set `self.LastSpeed` (`KismetMathLibrary.FInterpTo` (`self.LastSpeed`) 0.0 (`GameplayStatics.GetWorldDeltaSeconds`) 0.02)))
    (`SceneComponent.K2_AddRelativeLocation` (`self.Sphere`) (* (`self.GetActorForwardVector`) _output_get) true false)
    (else
      (`SceneComponent.K2_AddRelativeLocation` (`self.Sphere`) (* (`self.GetActorForwardVector`) _returnvalue) true false)
      (set `self.LastSpeed` _returnvalue))))

(fn `MoveVertical`
  (params (VerticalSpeed :type "Float (double-precision)"))
  (bind (_returnvalue_x _returnvalue_y) (`KismetMathLibrary.BreakVector` (`self.K2_GetActorLocation`)))
  (bind (_returnvalue_x_2 _returnvalue_y_2 _returnvalue_z) (`KismetMathLibrary.BreakVector` (`self.K2_GetActorLocation`)))
  (bind _maxheight (`self.MaxHeight`))
  (if (not (`self.Stopded`))
    (if (>= _returnvalue_z _maxheight)
      (`self.K2_SetActorLocation` (`KismetMathLibrary.MakeVector` _returnvalue_x _returnvalue_y _maxheight)))
    (`SceneComponent.K2_AddRelativeLocation` (`self.Sphere`) (* (`self.GetActorUpVector`) VerticalSpeed) false false)))

(fn `Rotate`
  (params (rotationAmount :type "Float (double-precision)"))
  (locals (NewLocalVar_0 :type "Rotator Structure" :default (struct)))
  (bind (_returnvalue_roll _returnvalue_pitch _returnvalue_yaw) (`KismetMathLibrary.BreakRotator` (`self.K2_GetActorRotation`)))
  (bind _player (`self.Player`))
  (bind _returnvalue (`SceneComponent.GetRelativeTransform` (`/Game/VirtualRealityBP/Blueprints/MotionControllerPawn.DefaultSceneRoot` _player)))
  (`SceneComponent.K2_SetWorldRotation` (`self.Sphere`) (`KismetMathLibrary.MakeRotator` (.roll (`self.K2_GetActorRotation`)) (.pitch (`self.K2_GetActorRotation`)) (+ (.yaw (`self.K2_GetActorRotation`)) rotationAmount)) false true)
  (if (not (`self.AntiMotionsickMode`))
    (set `self.xBack` (* (`KismetMathLibrary.Cos` (* (`self.GetGameTimeSinceCreation`) (`self.MoveSpeedX`))) (`self.MoveDistancex`)))
    (`self.K2_SetActorRelativeRotation` (`KismetMathLibrary.MakeRotator` (+ (`self.xBack`) (* rotationAmount 30.0)) _returnvalue_pitch _returnvalue_yaw))
    (`self.K2_AddActorLocalRotation` (`KismetMathLibrary.MakeRotator` 0.0 (* (`KismetMathLibrary.Cos` (* (`self.GetGameTimeSinceCreation`) (`self.MoveSpeedY`))) (`self.MoveDistancey`)) (* (`KismetMathLibrary.Cos` (* (`self.GetGameTimeSinceCreation`) (`self.MoveSpeedZ`))) (`self.MoveDistancez`))))
    (if (`self.NoWavesForPlayer`)
      (`self.K2_AddActorLocalRotation` (`self.Player`) (`KismetMathLibrary.MakeRotator` 0.0 (* (* (`KismetMathLibrary.Cos` (* (`self.GetGameTimeSinceCreation`) (`self.MoveSpeedY`))) (`self.MoveDistancey`)) -1.0) (* (* (`KismetMathLibrary.Cos` (* (`self.GetGameTimeSinceCreation`) (`self.MoveSpeedZ`))) (`self.MoveDistancez`)) -1.0)) false false)
      (`self.K2_SetActorRelativeRotation` _player (`KismetMathLibrary.MakeRotator` (* (`self.xBack`) -1.0) (.pitch (.rotation _returnvalue)) (.yaw (.rotation _returnvalue))) false false))))

(fn `UserConstructionScript`)

(fn `WaveMovement`)