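; BP_Creature is a creature that travels along a referenced spline while the player's ship is within its sphere trigger.
; On BeginPlay a timeline starts paused at a start offset, with its running rate derived from Duration.
; The timeline's alpha maps to spline distance, setting world location and rotation.
; Ship overlap restores the play rate; the ship or a CreatureStopVolume leaving the sphere zeroes it.
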(event `self.ReceiveBeginPlay`
  (set `self.NormalSpeed` (/ 1.0 (`self.Duration`)))
  (`self.SetUpTimeline`))

(event `self.ReceiveActorBeginOverlap`
  (params (OtherActor :type "Actor Object Reference")))

(event `self.SphereTrigger.OnComponentEndOverlap`
  (params (OverlappedComponent :type "PrimitiveComponent Object Reference") (OtherActor :type "Actor Object Reference") (OtherComp :type "PrimitiveComponent Object Reference") (OtherBodyIndex :type Integer))
  (`|ExecutionSequence`
    (:`then_0`
      (cast `/Game/Blueprints/BP_ShipController2` OtherActor))
    (:`then_1`
      (cast `/Game/Blueprints/CreatureStopVolume` OtherActor)))
  (`self.Stop`))

(event `self.SphereTrigger.OnComponentBeginOverlap`
  (params (OverlappedComponent :type "PrimitiveComponent Object Reference") (OtherActor :type "Actor Object Reference") (OtherComp :type "PrimitiveComponent Object Reference") (OtherBodyIndex :type Integer) (bFromSweep :type Boolean) (SweepResult :type "HitResult Structure (by ref)"))
  (cast `/Game/Blueprints/BP_ShipController2` OtherActor)
  (`self.Start`))

(event `Stop`
  (`KismetSystemLibrary.PrintString` "Left Magpie Trigger")
  (`TimelineComponent.SetPlayRate` (`self.CreatureMover`) 0.0))

(event `Start`
  (`KismetSystemLibrary.PrintString` "Entered Magpie Trigger")
  (`TimelineComponent.SetPlayRate` (`self.CreatureMover`) (`self.NormalSpeed`)))

(event `SetUpTimeline`
  (bind _returnvalue (`KismetMathLibrary.Lerp` 0.0 (`SplineComponent.GetSplineLength` (`/Game/Blueprints/BP_CreatureSpline.Spline` (`self.SplineReference`))) (`self.Alpha`)))
  (`TimelineComponent.SetPlayRate` (`self.CreatureMover`) 0.0)
  (`TimelineComponent.SetNewTime` (`self.CreatureMover`) (`self.CreatureStartOffset`))
  (bind (_direction _alpha) (`Timeline|CreatureMover`)
    (:`Update`
      (set `self.Alpha` _alpha)
      (`self.K2_SetActorLocationAndRotation` (`SplineComponent.GetLocationAtDistanceAlongSpline` (`/Game/Blueprints/BP_CreatureSpline.Spline` (`self.SplineReference`)) _returnvalue "World") (`SplineComponent.GetRotationAtDistanceAlongSpline` (`/Game/Blueprints/BP_CreatureSpline.Spline` (`self.SplineReference`)) _returnvalue "World")))))

(fn `NewFunction_0`)

(fn `UserConstructionScript`)