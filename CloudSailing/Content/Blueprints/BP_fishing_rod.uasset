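; VR fishing rod that a motion controller picks up and that re-attaches to the ship when dropped.
; Tick moves the bait along the cable particles to its end and, while CanThrow is set, triggers a throw on fast rod movement.
; The throw sequence pays out cable, spawns a BP_Fish_v2 at the bait attached to the rod, then reels back in using timed delays and a FlipFlop.
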(event `Motion_Throw`
  (`/Engine/EditorBlueprintResources/StandardMacros.DoOnce` false :!label _label
    (:`Completed`
      (`/Engine/EditorBlueprintResources/StandardMacros.FlipFlop` :!label _label_2
        (:`A`
          (set `self.throw` true)
          (set `self.throwSpeed` 20.0)
          (set `CableComponent.CableForce` (0.0 0.0 0.0) (`self.Cable`))
          (`KismetSystemLibrary.Delay` 1.0)
          (set `self.throw` false)
          (`KismetSystemLibrary.Delay` 3.0)
          (bind _returnvalue (`|SpawnActorFromClass` "/Game/Blueprints/BP_Fish_v2.BP_Fish_v2_C" (`KismetMathLibrary.MakeTransform` (`SceneComponent.K2_GetComponentLocation` (`self.Bait`))) "Undefined" "OverrideRootScale" null null))
          (`/Game/Blueprints/BP_Fish_v2.AttachToRod` _returnvalue self)
          (`KismetSystemLibrary.Delay` 2.0)
          (goto _label_2))
        (:`B`
          (set `self.throw` true)
          (set `self.throwSpeed` -4.0)
          (`KismetSystemLibrary.Delay` 5.0)
          (set `self.throw` false)
          (set `CableComponent.CableForce` (0.0 0.0 0.0) (`self.Cable`))
          (goto _label :!via `Reset`))))))

(event `Throw_event`)

(event `self.ReceiveBeginPlay`
  (bind _outactors (`GameplayStatics.GetAllActorsOfClass` "/Game/Blueprints/BP_ShipController2.BP_ShipController2_C"))
  (set `self.Ship` (`|GetArrayItem` _outactors))
  (`KismetSystemLibrary.Delay` 0.2)
  (`self.K2_AttachToComponent` (`/Game/Blueprints/BP_ShipController2.Sphere` (`self.Ship`)) "None" "KeepWorld" "KeepWorld" "KeepWorld" false))

(event `self.ReceiveTick`
  (params (DeltaSeconds :type "Float (single-precision)"))
  (bind _cable (`self.Cable`))
  (bind _returnvalue (`SceneComponent.K2_GetComponentLocation` (`self.rod`)))
  (`|ExecutionSequence`
    (:`then_0`
      (for _array_element (`CableComponent.GetCableParticleLocations` _cable)
        (`SceneComponent.K2_SetWorldLocation` (`self.Bait`) _array_element false false))
      (if (`self.throw`)
        (set `CableComponent.CableLength` (+ (`CableComponent.CableLength` _cable) (`self.throwSpeed`)) _cable)))
    (:`then_1`
      (if (`self.canThrow`)
        (set `self.ThrowForce` (`KismetMathLibrary.VSize` (- _returnvalue (`self.lastThrowForce`))))
        (set `self.lastThrowForce` _returnvalue)
        (if (< 20.0 (`self.ThrowForce`))
          (`|ExecutionSequence`
            (:`then_0`
              (`/Engine/EditorBlueprintResources/StandardMacros.DoOnce` true :!label _label_3
                (:`Completed`
                  (`self.Motion_Throw`))))
            (:`then_1`
              (goto _label_3 :!via `Reset`))))))))

(event `/Game/VirtualRealityBP/Blueprints/PickupActorInterface.Pickup`
  (params (AttachTo :type "SceneComponent Object Reference") (PH :type "PhysicsHandleComponent Object Reference") (BoneName :type Name) (Hand :type "EControllerHand Enum" :default "Left"))
  (`self.K2_DetachFromActor` "KeepWorld" "KeepWorld" "KeepWorld")
  (`PrimitiveComponent.SetSimulatePhysics` (`self.rod`) false)
  (`SceneComponent.K2_AttachToComponent` (`self.K2_GetRootComponent`) AttachTo "None" "KeepWorld" "KeepWorld" "KeepWorld" false))

(event `/Game/VirtualRealityBP/Blueprints/PickupActorInterface.Drop`
  (params (Hand :type "EControllerHand Enum" :default "Left"))
  (`PrimitiveComponent.SetSimulatePhysics` (`self.rod`) false)
  (`self.K2_DetachFromActor` "KeepWorld" "KeepWorld" "KeepWorld")
  (`self.K2_AttachToComponent` (`/Game/Blueprints/BP_ShipController2.Sphere` (`self.Ship`)) "None" "KeepWorld" "KeepWorld" "KeepWorld" false))

(fn `UserConstructionScript`)