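; Grabbable fish that can be picked up by hand, thrown, or hung on a fishing rod.
; Pickup grabs the rig's main bone through the passed-in physics handle with very stiff settings; drop by the holding hand softens them, delays restoring query collision, and flags it thrown briefly.
; At start it stops simulating and attaches to the ship's sphere; in rod mode, Tick snaps it to the bait's transform.
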(event `/Game/VirtualRealityBP/Blueprints/PickupActorInterface.Pickup`
  (params (AttachTo :type "SceneComponent Object Reference") (PH :type "PhysicsHandleComponent Object Reference") (BoneName :type Name) (Hand :type "EControllerHand Enum" :default "Left"))
  (bind (_returnvalue_location _returnvalue_rotation) (`KismetMathLibrary.BreakTransform` (`SceneComponent.K2_GetComponentToWorld` AttachTo)))
  (bind _fish_rig (`self.fish_rig`))
  (`PrimitiveComponent.SetSimulatePhysics` (`self.fish_rig`) true)
  (`PhysicsHandleComponent.SetLinearDamping` PH 0.0)
  (`PhysicsHandleComponent.SetLinearStiffness` PH 1500000.0)
  (`PhysicsHandleComponent.SetAngularDamping` PH 0.0)
  (`PhysicsHandleComponent.SetAngularStiffness` PH 1500000.0)
  (set `PhysicsHandleComponent.bInterpolateTarget` false PH)
  (if (`self.graped`)
    (`PhysicsHandleComponent.ReleaseComponent` (`self.PH`)))
  (set `self.GrappedHand` Hand)
  (set `self.graped` true)
  (set `self.PH` PH)
  (`PhysicsHandleComponent.GrabComponentAtLocationWithRotation` PH (`self.fish_rig`) "jt_main" _returnvalue_location _returnvalue_rotation)
  (`PrimitiveComponent.SetCollisionEnabled` _fish_rig "PhysicsOnly")
  (`PrimitiveComponent.SetCollisionResponseToAllChannels` _fish_rig "ECR_Overlap")
  (`PrimitiveComponent.SetEnableGravity` (`self.fish_rig`) true))

(event `/Game/VirtualRealityBP/Blueprints/PickupActorInterface.Drop`
  (params (Hand :type "EControllerHand Enum" :default "Left"))
  (bind _ph (`self.PH`))
  (if (`|EnumEquality` (`self.GrappedHand`) Hand)
    (`PhysicsHandleComponent.SetLinearDamping` _ph 20.0)
    (`PhysicsHandleComponent.SetLinearStiffness` _ph 300.0)
    (`PhysicsHandleComponent.SetAngularDamping` _ph 50.0)
    (`PhysicsHandleComponent.SetAngularStiffness` _ph 150.0)
    (set `PhysicsHandleComponent.bInterpolateTarget` true _ph)
    (set `self.thrown` true)
    (set `self.graped` false)
    (`PhysicsHandleComponent.ReleaseComponent` (`self.PH`))
    (`PrimitiveComponent.SetEnableGravity` (`self.fish_rig`) true)
    (`KismetSystemLibrary.Delay` 0.2)
    (`PrimitiveComponent.SetCollisionEnabled` (`self.fish_rig`) "QueryAndPhysics")
    (`PrimitiveComponent.SetCollisionResponseToAllChannels` (`self.fish_rig`) "ECR_Overlap")
    (`PrimitiveComponent.SetCollisionResponseToChannel` (`self.fish_rig`) "ECC_WorldStatic" "ECR_Block")
    (`KismetSystemLibrary.Delay` 5.0)
    (set `self.thrown` false)))

(event `self.ReceiveBeginPlay`
  (bind _outactors (`GameplayStatics.GetAllActorsOfClass` "/Game/Blueprints/BP_ShipController2.BP_ShipController2_C"))
  (set `self.Ship` (`|GetArrayItem` _outactors))
  (`PrimitiveComponent.SetSimulatePhysics` (`self.fish_rig`) false)
  (`KismetSystemLibrary.Delay` 0.2)
  (`self.K2_AttachToComponent` (`/Game/Blueprints/BP_ShipController2.Sphere` (`self.Ship`)) "None" "KeepWorld" "KeepWorld" "KeepWorld" false))

(event `AttachToRod`
  (params (FishingRod :type "/Game/Blueprints/BP_fishing_rod Object Reference"))
  (set `self.FishingRod` FishingRod)
  (set `self.FishRodMode` true))

(event `self.ReceiveTick`
  (params (DeltaSeconds :type "Float (single-precision)"))
  (bind _bait (`/Game/Blueprints/BP_fishing_rod.Bait` (`self.FishingRod`)))
  (if (`self.FishRodMode`)
    (`self.K2_SetActorLocationAndRotation` (`SceneComponent.K2_GetComponentLocation` _bait) (`SceneComponent.K2_GetComponentRotation` _bait))))

(fn `UserConstructionScript`)