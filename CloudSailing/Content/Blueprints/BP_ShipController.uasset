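; BP_ShipController is a Blueprint that drives a ship's Cube component with simple keyboard movement.
; X sets forward speed while held, and Y and C set counter-clockwise and clockwise yaw speed, each resetting to zero on release.
; Every Tick, MoveForward offsets the Cube along the actor's forward vector and Rotate sets its world yaw from the actor's rotation, both swept and per frame without delta-time scaling.
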(event `self.ReceiveBeginPlay`)

(event `self.ReceiveTick`
  (params (DeltaSeconds :type "Float (single-precision)"))
  (`self.MoveForward` (`self.Speed`))
  (`self.Rotate` (`self.RotationSpeed`)) ; Positive Rotation Amount: CW\nNegative Rotation Amount: CCW
)

(event `Key|X`
  (params (Key :type "Key Structure"))
  (:`Pressed`
    (set `self.Speed` 1.0))
  (:`Released`
    (set `self.Speed` 0.0)))

(event `Key|Y`
  (params (Key :type "Key Structure"))
  (:`Pressed`
    (set `self.RotationSpeed` -1.0))
  (:`Released`
    (set `self.RotationSpeed` 0.0)))

(event `Key|C`
  (params (Key :type "Key Structure"))
  (:`Pressed`
    (set `self.RotationSpeed` 1.0))
  (:`Released`
    (set `self.RotationSpeed` 0.0)))

(fn `MoveForward`
  (params (ForwardSpeed :type "Float (double-precision)"))
  (`SceneComponent.K2_AddRelativeLocation` (`self.Cube`) (* (`self.GetActorForwardVector`) ForwardSpeed) true false))

(fn `Rotate`
  (params (rotationAmount :type "Float (double-precision)"))
  (locals (NewLocalVar_0 :type "Rotator Structure" :default (struct)))
  (`SceneComponent.K2_SetWorldRotation` (`self.Cube`) (`KismetMathLibrary.MakeRotator` (.roll (`self.K2_GetActorRotation`)) (.pitch (`self.K2_GetActorRotation`)) (+ (.yaw (`self.K2_GetActorRotation`)) rotationAmount)) true false))

(fn `UserConstructionScript`)