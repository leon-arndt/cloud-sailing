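; SpeedRope is a grabbable pull-rope throttle that sets the speed of the ship (BP_ShipController2).
; On BeginPlay it moves to the first ship's SpeedCube and attaches to its Sphere.
; Pickup and Drop, part of motion-controller grabbing, attach CubeEnd to the hand or back to the root.
; Tick derives ship speed from the CubeStart–CubeEnd distance plus Height, and eases the released handle back to rest.
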(event `self.ReceiveBeginPlay`
  (bind _speedcube (`/Game/Blueprints/BP_ShipController2.speedCube` (`self.Ship`)))
  (bind _outactors (`GameplayStatics.GetAllActorsOfClass` "/Game/Blueprints/BP_ShipController2.BP_ShipController2_C"))
  (set `self.ship` (`|GetArrayItem` _outactors))
  (`self.K2_SetActorLocationAndRotation` (`SceneComponent.K2_GetComponentLocation` _speedcube) (`SceneComponent.K2_GetComponentRotation` _speedcube))
  (`self.K2_AttachToComponent` (`/Game/Blueprints/BP_ShipController2.Sphere` (`self.Ship`)) "None" "KeepWorld" "KeepWorld" "KeepWorld"))

(event `/Game/VirtualRealityBP/Blueprints/PickupActorInterface.Pickup`
  (params (AttachTo :type "SceneComponent Object Reference") (PH :type "PhysicsHandleComponent Object Reference") (BoneName :type Name) (Hand :type "EControllerHand Enum" :default "Left"))
  (bind _cubeend (`self.CubeEnd`))
  (`PrimitiveComponent.SetSimulatePhysics` _cubeend false)
  (set `self.grapped` true)
  (`SceneComponent.K2_AttachToComponent` _cubeend AttachTo "None" "KeepWorld" "KeepWorld" "KeepWorld" false))

(event `/Game/VirtualRealityBP/Blueprints/PickupActorInterface.Drop`
  (params (Hand :type "EControllerHand Enum" :default "Left"))
  (set `self.grapped` false)
  (`PrimitiveComponent.SetSimulatePhysics` (`self.CubeEnd`) false)
  (`SceneComponent.K2_AttachToComponent` (`self.CubeEnd`) (`self.DefaultSceneRoot`) "None" "KeepWorld" "KeepWorld" "KeepWorld" false))

(event `self.ReceiveTick`
  (params (DeltaSeconds :type "Float (single-precision)"))
  (bind _cubeend (`self.CubeEnd`))
  (`|ExecutionSequence`
    (:`then_0`
      (if (not (`self.grapped`))
        (`SceneComponent.K2_SetRelativeLocation` _cubeend (`KismetMathLibrary.VInterpTo` (`SceneComponent.RelativeLocation` _cubeend) (`KismetMathLibrary.MakeVector` 0.0 0.0 (`self.Height`)) (`GameplayStatics.GetWorldDeltaSeconds`) 3.0) false false)
        (`SceneComponent.K2_SetRelativeRotation` _cubeend (`KismetMathLibrary.RInterpTo` (`SceneComponent.RelativeRotation` _cubeend) (struct :`Yaw` 90.0) (`GameplayStatics.GetWorldDeltaSeconds`) 3.0) false false))
      (set `/Game/Blueprints/BP_ShipController2.Speed` (* (+ (`KismetMathLibrary.VSize` (- (`SceneComponent.K2_GetComponentLocation` (`self.CubeEnd`)) (`SceneComponent.K2_GetComponentLocation` (`self.CubeStart`)))) (`self.Height`)) 0.45) (`self.ship`)))))

(fn `UserConstructionScript`
  (`SceneComponent.K2_SetRelativeLocation` (`self.CubeEnd`) (`KismetMathLibrary.MakeVector` 0.0 0.0 (`self.Height`)) false false))