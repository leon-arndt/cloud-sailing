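; A grabbable VR throttle for BP_ShipController2 that sets either its Speed or its VerticalSpeed, depending on VerticalMode.
; On BeginPlay it attaches to the ship's sphere, and while held by a motion controller its mesh follows the hand on world Z only.
; Its height offset from the ship's matching SpeedCube, minus a dead zone, becomes a target the ship value eases toward with FInterpTo.
; When released it snaps back to that cube's height, easing the value to zero.
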(event `self.ReceiveBeginPlay`
  (bind _outactors (`GameplayStatics.GetAllActorsOfClass` "/Game/Blueprints/BP_ShipController2.BP_ShipController2_C"))
  (set `self.ship` (`|GetArrayItem` _outactors))
  (`self.K2_AttachToComponent` (`/Game/Blueprints/BP_ShipController2.Sphere` (`self.Ship`)) "None" "KeepWorld" "KeepWorld" "KeepWorld"))

(event `self.ReceiveTick`
  (params (DeltaSeconds :type "Float (single-precision)"))
  (bind _staticmeshcomponent (`self.StaticMeshComponent`))
  (bind _speed (`self.speed`))
  (bind _staticmeshcomponent_2 (`self.StaticMeshComponent`))
  (bind _ship (`self.ship`))
  (bind _ship_2 (`self.ship`))
  (bind (_returnvalue_x _returnvalue_y _returnvalue_z) (`KismetMathLibrary.BreakVector` (`SceneComponent.K2_GetComponentLocation` (`self.StaticMeshComponent`))))
  (bind (_returnvalue_x_2 _returnvalue_y_2) (`KismetMathLibrary.BreakVector` (`SceneComponent.K2_GetComponentLocation` _staticmeshcomponent)))
  (bind (_returnvalue_x_3 _returnvalue_y_3 _returnvalue_z_2) (`KismetMathLibrary.BreakVector` (`SceneComponent.K2_GetComponentLocation` (`self.Hand`))))
  (bind (_returnvalue_x_4 _returnvalue_y_4) (`KismetMathLibrary.BreakVector` (`SceneComponent.K2_GetComponentLocation` _staticmeshcomponent_2)))
  (bind (_returnvalue_x_5 _returnvalue_y_5 _returnvalue_z_3) (`KismetMathLibrary.BreakVector` (`SceneComponent.K2_GetComponentLocation` (select `bool` (`self.VerticalMode`) :`false` (`/Game/Blueprints/BP_ShipController2.speedCube` _ship) :`true` (`/Game/Blueprints/BP_ShipController2.speedCube1` _ship)))))
  (bind (_returnvalue_x_6 _returnvalue_y_6 _returnvalue_z_4) (`KismetMathLibrary.BreakVector` (`SceneComponent.K2_GetComponentLocation` (select `bool` (`self.VerticalMode`) :`false` (`/Game/Blueprints/BP_ShipController2.speedCube` _ship_2) :`true` (`/Game/Blueprints/BP_ShipController2.speedCube1` _ship_2)))))
  (bind _returnvalue (select `bool` (< (`KismetMathLibrary.Abs` _speed) 5.0) :`false` (select `bool` (< (`self.speed`) 0.0) :`false` (- _speed 5.0) :`true` (+ _speed 5.0))))
  (if (`self.grabed`)
    (`SceneComponent.K2_SetWorldLocation` _staticmeshcomponent (`KismetMathLibrary.MakeVector` _returnvalue_x_2 _returnvalue_y_2 (+ _returnvalue_z_2 (`self.distanceToCube`))) false false)
    (set `self.speed` (* (- _returnvalue_z_3 _returnvalue_z) -1.0))
    (else
      (`SceneComponent.K2_SetWorldLocation` _staticmeshcomponent_2 (`KismetMathLibrary.MakeVector` _returnvalue_x_4 _returnvalue_y_4 _returnvalue_z_4) false false)
      (set `self.speed` 0.0)))
  (if (`self.VerticalMode`)
    (set `/Game/Blueprints/BP_ShipController2.VerticalSpeed` (`KismetMathLibrary.FInterpTo` (`/Game/Blueprints/BP_ShipController2.VerticalSpeed` (`self.ship`)) (* _returnvalue 1.0) (`GameplayStatics.GetWorldDeltaSeconds`) 0.8) (`self.ship`))
    (else
      (set `/Game/Blueprints/BP_ShipController2.Speed` (`KismetMathLibrary.FInterpTo` (`/Game/Blueprints/BP_ShipController2.Speed` (`self.ship`)) (* _returnvalue -1.0) (`GameplayStatics.GetWorldDeltaSeconds`) 0.8) (`self.ship`)))))

(event `/Game/VirtualRealityBP/Blueprints/PickupActorInterface.Pickup`
  (params (AttachTo :type "SceneComponent Object Reference") (PH :type "PhysicsHandleComponent Object Reference") (BoneName :type Name) (Hand :type "EControllerHand Enum" :default "Left"))
  (bind (_returnvalue_x _returnvalue_y _returnvalue_z) (`KismetMathLibrary.BreakVector` (`SceneComponent.K2_GetComponentLocation` (`self.StaticMeshComponent`))))
  (bind (_returnvalue_x_2 _returnvalue_y_2 _returnvalue_z_2) (`KismetMathLibrary.BreakVector` (`SceneComponent.K2_GetComponentLocation` (`self.Hand`))))
  (bind (_returnvalue_x_3 _returnvalue_y_3 _returnvalue_z_3) (`KismetMathLibrary.BreakVector` (`SceneComponent.K2_GetComponentLocation` (`self.Hand`))))
  (set `self.Hand` AttachTo)
  (set `self.grabed` true)
  (set `self.distanceToCube` (- _returnvalue_z _returnvalue_z_2))
  (set `self.handStartZ` (- (+ _returnvalue_z_3 (`self.distanceToCube`)) (`self.speed`))))

(event `/Game/VirtualRealityBP/Blueprints/PickupActorInterface.Drop`
  (params (Hand :type "EControllerHand Enum" :default "Left"))
  (set `self.grabed` false))

(fn `UserConstructionScript`)