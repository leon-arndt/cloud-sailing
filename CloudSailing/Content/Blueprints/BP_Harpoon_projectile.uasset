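; BP_Harpoon_projectile is a harpoon spear projectile that sticks into whatever it hits.
; Fire enables physics on the spear mesh, launches it along the root's forward vector, ignoring its Direction input, and destroys the actor after a delay.
; On hit, the spear stops simulating, drops collision and attaches to the struck component, keeping its world transform.
; A node that would align it to the impact normal is disconnected.
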(event `Fire`
  (params (Direction :type "Vector Structure"))
  (bind _harpoon_edit_harpoon_blocking_moveable_harpoon_speer (`self.Harpoon_edit_harpoon_blocking_moveable_harpoon_speer`))
  (`PrimitiveComponent.SetSimulatePhysics` _harpoon_edit_harpoon_blocking_moveable_harpoon_speer true)
  (`PrimitiveComponent.SetPhysicsLinearVelocity` _harpoon_edit_harpoon_blocking_moveable_harpoon_speer (* (`SceneComponent.GetForwardVector` (`self.DefaultSceneRoot`)) 2000.0) false "None")
  (`KismetSystemLibrary.Delay` 5.0)
  (`self.K2_DestroyActor`))

(event `self.Harpoon_edit_harpoon_blocking_moveable_harpoon_speer.OnComponentHit`
  (params (HitComponent :type "PrimitiveComponent Object Reference") (OtherActor :type "Actor Object Reference") (OtherComp :type "PrimitiveComponent Object Reference") (NormalImpulse :type "Vector Structure") (Hit :type "HitResult Structure (by ref)"))
  (`PrimitiveComponent.SetSimulatePhysics` (`self.Harpoon_edit_harpoon_blocking_moveable_harpoon_speer`) false)
  (`PrimitiveComponent.SetCollisionEnabled` (`self.Harpoon_edit_harpoon_blocking_moveable_harpoon_speer`) "NoCollision")
  (`SceneComponent.K2_AttachToComponent` (`self.Harpoon_edit_harpoon_blocking_moveable_harpoon_speer`) (`.HitComponent` (`GameplayStatics.BreakHitResult` Hit)) "None" "KeepWorld" "KeepWorld" "KeepWorld" true))

(fn `UserConstructionScript`)