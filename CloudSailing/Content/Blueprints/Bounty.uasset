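; Bounty is a pickup-style actor that bobs in place until it is hit, then gets reeled toward the player ship.
; On BeginPlay it finds the first BP_ShipController2 and attaches to that ship's Sphere, keeping its world transform.
; Each Tick oscillates the Cube with per-axis cosine offsets until a component hit sets Hit.
; After that, it disables Cube collision and moves at constant speed toward a point above the Sphere.
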(event `self.ReceiveBeginPlay`
  (bind _outactors (`GameplayStatics.GetAllActorsOfClass` "/Game/Blueprints/BP_ShipController2.BP_ShipController2_C"))
  (set `self.Ship` (`|GetArrayItem` _outactors))
  (`self.K2_AttachToComponent` (`/Game/Blueprints/BP_ShipController2.Sphere` (`self.Ship`)) "None" "KeepWorld" "KeepWorld" "KeepWorld" false))

(event `self.ReceiveTick`
  (params (DeltaSeconds :type "Float (single-precision)"))
  (if (`self.Hit`)
    (`self.K2_SetActorLocation` (`KismetMathLibrary.VInterpTo_Constant` (`self.K2_GetActorLocation`) (+ (`SceneComponent.K2_GetComponentLocation` (`/Game/Blueprints/BP_ShipController2.Sphere` (`self.Ship`))) (0.0 0.0 100.0)) (`GameplayStatics.GetWorldDeltaSeconds`) 200.0))
    (`PrimitiveComponent.SetCollisionEnabled` (`self.Cube`) "NoCollision")
    (else
      (`SceneComponent.K2_AddRelativeLocation` (`self.Cube`) (* (`KismetMathLibrary.MakeVector` (`KismetMathLibrary.Cos` (* (`self.GetGameTimeSinceCreation`) (`self.MoveSpeedX`))) (`KismetMathLibrary.Cos` (* (`self.GetGameTimeSinceCreation`) (`self.MoveSpeedY`))) (`KismetMathLibrary.Cos` (* (`self.GetGameTimeSinceCreation`) (`self.MoveSpeedZ`)))) (/ (`self.MoveDistance`) 2.0)) false false))))

(event `self.Cube.OnComponentHit`
  (params (HitComponent :type "PrimitiveComponent Object Reference") (OtherActor :type "Actor Object Reference") (OtherComp :type "PrimitiveComponent Object Reference") (NormalImpulse :type "Vector Structure") (Hit :type "HitResult Structure (by ref)"))
  (set `self.Hit` true))

(fn `UserConstructionScript`)