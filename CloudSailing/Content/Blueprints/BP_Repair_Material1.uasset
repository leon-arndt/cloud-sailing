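; BP_Repair_Material1 is a grabbable physics prop, named as a repair material, for VR motion-controller interaction.
; On BeginPlay it finds the first BP_ShipController2 and attaches to that ship's Sphere, keeping its world transform.
; Pickup turns off mesh physics and attaches the root to the supplied component.
; Drop restores physics and detaches the actor without reattaching it to the ship.
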(event `self.ReceiveBeginPlay`
  (bind _outactors (`GameplayStatics.GetAllActorsOfClass` "/Game/Blueprints/BP_ShipController2.BP_ShipController2_C"))
  (set `self.Ship` (`|GetArrayItem` _outactors))
  (`self.K2_AttachToComponent` (`/Game/Blueprints/BP_ShipController2.Sphere` (`self.Ship`)) "None" "KeepWorld" "KeepWorld" "KeepWorld" false))

(event `/Game/VirtualRealityBP/Blueprints/PickupActorInterface.Pickup`
  (params (AttachTo :type "SceneComponent Object Reference") (PH :type "PhysicsHandleComponent Object Reference") (BoneName :type Name) (Hand :type "EControllerHand Enum" :default "Left"))
  (`KismetSystemLibrary.PrintString` "cube_grapped")
  (`PrimitiveComponent.SetSimulatePhysics` (`self.StaticMeshComponent`) false)
  (`SceneComponent.K2_AttachToComponent` (`self.K2_GetRootComponent`) AttachTo "None" "KeepWorld" "KeepWorld" "KeepWorld" false))

(event `/Game/VirtualRealityBP/Blueprints/PickupActorInterface.Drop`
  (params (Hand :type "EControllerHand Enum" :default "Left"))
  (`PrimitiveComponent.SetSimulatePhysics` (`self.StaticMeshComponent`) true)
  (`self.K2_DetachFromActor` "KeepWorld" "KeepWorld" "KeepWorld"))

(fn `UserConstructionScript`)