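; Flying enemy that circles and attacks the player ship, and can be diverted by a thrown fish.
; A Tick-driven state switch moves it with interpolated positions and turns its mesh along its movement.
; See_range starts circling, then a delayed attack spawns BP_ship_Damage attached to the ship before fleeing.
; Thrown fish in FishCatchRadius trigger a brief chase before fleeing; Cube overlap grabs the fish, which is carried at Scene.
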(event `self.ReceiveTick`
  (params (DeltaSeconds :type "Float (single-precision)"))
  (bind (_returnvalue_roll _returnvalue_pitch _returnvalue_yaw) (`KismetMathLibrary.BreakRotator` (`KismetMathLibrary.Conv_VectorToRotator` (- (`self.K2_GetActorLocation`) (`self.lastLocation`)))))
  (bind (_returnvalue_location _returnvalue_rotation) (`KismetMathLibrary.BreakTransform` (`SceneComponent.K2_GetComponentToWorld` (`/Game/Blueprints/BP_ShipController2.attackLocation1` (`self.Ship`)))))
  (bind _returnvalue_location_2 (`KismetMathLibrary.BreakTransform` (`SceneComponent.GetSocketTransform` (`/Game/Blueprints/BP_Fish_v2.fish_rig` (`self.Fish`)) "jt_main" "RTS_World")))
  (if (`self.full`)
    (`SceneComponent.K2_SetWorldLocation` (`/Game/Blueprints/BP_Fish_v2.fish_rig` (`self.Fish`)) (`SceneComponent.K2_GetComponentLocation` (`self.Scene`)) false false))
  ;[1 1 1] rotate towards movement
  (`SceneComponent.K2_SetWorldRotation` (`self.SkeletalMesh`) (`KismetMathLibrary.RInterpTo` (`SceneComponent.K2_GetComponentRotation` (`self.SkeletalMesh`)) (`KismetMathLibrary.MakeRotator` _returnvalue_roll _returnvalue_pitch (- _returnvalue_yaw 90.0)) (`GameplayStatics.GetWorldDeltaSeconds`) 1.0) false false)
  (set `self.lastLocation` (`self.K2_GetActorLocation`))
  (switch `/Game/Blueprints/Enemy_State` (`self.State`)
    (:`NewEnumerator1`
      (set `self.CircularPossition` (+ (`self.CircularPossition`) (`self.CircularSpeed`)))
      (`self.K2_SetActorLocation` (`KismetMathLibrary.VInterpTo` (`self.K2_GetActorLocation`) (+ (* (`KismetMathLibrary.GetForwardVector` (`KismetMathLibrary.MakeRotator` 0.0 35.0 (`self.CircularPossition`))) 1000.0) (`self.K2_GetActorLocation` (`self.Ship`))) (`GameplayStatics.GetWorldDeltaSeconds`) (`self.FlySpeed`)) true))
    (:`NewEnumerator4`
      (if (not (`self.full`))
        (`self.K2_SetActorLocation` (`KismetMathLibrary.VInterpTo` (`self.K2_GetActorLocation`) _returnvalue_location_2 (`GameplayStatics.GetWorldDeltaSeconds`) 5.0) true)))
    (:`NewEnumerator2`
      (`self.K2_SetActorLocation` (`KismetMathLibrary.VInterpTo` (`self.K2_GetActorLocation`) (`SceneComponent.K2_GetComponentLocation` (`/Game/Blueprints/BP_ShipController2.attackLocation1` (`self.Ship`))) (`GameplayStatics.GetWorldDeltaSeconds`) 2.0) true)
      (`KismetSystemLibrary.Delay` 2.0)
      (bind _returnvalue (`|SpawnActorFromClass` "/Game/Blueprints/BP_ship_Damage.BP_ship_Damage_C" (`KismetMathLibrary.MakeTransform` _returnvalue_location _returnvalue_rotation) "Undefined" "OverrideRootScale" null null))
      (`/Game/Blueprints/BP_ship_Damage.AttachToShip` _returnvalue (`self.Ship`))
      (set `self.State` "NewEnumerator3"))
    (:`NewEnumerator3`
      (`self.K2_SetActorLocation` (`KismetMathLibrary.VInterpTo` (`self.K2_GetActorLocation`) (+ (* (`KismetMathLibrary.GetForwardVector` (`KismetMathLibrary.MakeRotator` 0.0 10.0 (`self.CircularPossition`))) 5000.0) (`self.K2_GetActorLocation` (`self.Ship`))) (`GameplayStatics.GetWorldDeltaSeconds`) 0.05) true))))

(event `self.ReceiveBeginPlay`
  (bind _outactors (`GameplayStatics.GetAllActorsOfClass` "/Game/Blueprints/BP_ShipController2.BP_ShipController2_C"))
  (set `self.Ship` (`|GetArrayItem` _outactors)))

(event `self.See_range.OnComponentBeginOverlap`
  (params (OverlappedComponent :type "PrimitiveComponent Object Reference") (OtherActor :type "Actor Object Reference") (OtherComp :type "PrimitiveComponent Object Reference") (OtherBodyIndex :type Integer) (bFromSweep :type Boolean) (SweepResult :type "HitResult Structure (by ref)"))
  (`/Engine/EditorBlueprintResources/StandardMacros.DoOnce` false
    (:`Completed`
      (set `self.State` "NewEnumerator1")
      (`KismetSystemLibrary.Delay` (`self.AttackWaitTime`))
      (switch `/Game/Blueprints/Enemy_State` (`self.State`)
        (:`NewEnumerator1`
          (set `self.State` "NewEnumerator2"))))))

(event `self.FishCatchRadius.OnComponentBeginOverlap`
  (params (OverlappedComponent :type "PrimitiveComponent Object Reference") (OtherActor :type "Actor Object Reference") (OtherComp :type "PrimitiveComponent Object Reference") (OtherBodyIndex :type Integer) (bFromSweep :type Boolean) (SweepResult :type "HitResult Structure (by ref)"))
  (bind _asbp_fish_v_2 (cast `/Game/Blueprints/BP_Fish_v2` OtherActor))
  (if (`/Game/Blueprints/BP_Fish_v2.thrown` _asbp_fish_v_2)
    (set `self.State` "NewEnumerator4")
    (set `self.Fish` _asbp_fish_v_2)
    (`KismetSystemLibrary.Delay` 1.5)
    (set `self.State` "NewEnumerator3")))

(event `self.Cube.OnComponentBeginOverlap`
  (params (OverlappedComponent :type "PrimitiveComponent Object Reference") (OtherActor :type "Actor Object Reference") (OtherComp :type "PrimitiveComponent Object Reference") (OtherBodyIndex :type Integer) (bFromSweep :type Boolean) (SweepResult :type "HitResult Structure (by ref)"))
  (bind _asbp_fish_v_2 (cast `/Game/Blueprints/BP_Fish_v2` OtherActor))
  (if (`/Game/Blueprints/BP_Fish_v2.thrown` _asbp_fish_v_2)
    (set `self.Fish` _asbp_fish_v_2)
    (set `self.full` true)
    (`PrimitiveComponent.SetSimulatePhysics` (`/Game/Blueprints/BP_Fish_v2.fish_rig` _asbp_fish_v_2) false)))

(fn `UserConstructionScript`)